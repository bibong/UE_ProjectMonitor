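; AC_Rotation is an actor component that spins its owner around the yaw axis while its Play flag is set, then returns it to its starting orientation.
; Tick applies a constant-speed world rotation and accumulates elapsed time.
; Once the duration has passed, it keeps spinning until the yaw is within Epsilon of the rotation cached at BeginPlay, then snaps to it, clears Play and resets the timer.
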(event `self.ReceiveBeginPlay`
  (set `self.InitialRotator` (`Actor.K2_GetActorRotation` (`self.GetOwner`))))

(event `self.ReceiveTick`
  (params (DeltaSeconds :type "Float (single-precision)"))
  (bind (_initialrotator_roll _initialrotator_pitch _initialrotator_yaw) (`KismetMathLibrary.BreakRotator` (`self.InitialRotator`)))
  (bind (_returnvalue_roll _returnvalue_pitch _returnvalue_yaw) (`KismetMathLibrary.BreakRotator` (`Actor.K2_GetActorRotation` (`self.GetOwner`))))
  (if (`self.bPlay`)
    (bind _output_get (set `self.ElapsedTime` (+ DeltaSeconds (`self.ElapsedTime`) 0.0)))
    (if (< _output_get (`self.RotationDuration`))
      (`Actor.K2_AddActorWorldRotation` (`self.GetOwner`) (`KismetMathLibrary.MakeRotator` 0.0 0.0 (* (`self.RotationSpeed`) DeltaSeconds)) false false)
      (else
        (`Actor.K2_AddActorWorldRotation` (`self.GetOwner`) (`KismetMathLibrary.MakeRotator` 0.0 0.0 (* (`self.RotationSpeed`) DeltaSeconds)) false false)
        (bind _output_get_2 (set `self.bPlay` (> (`KismetMathLibrary.Abs` (- _returnvalue_yaw _initialrotator_yaw)) (`self.Epsilon`))))
        (if (not _output_get_2)
          (`Actor.K2_SetActorRotation` (`self.GetOwner`) (`self.InitialRotator`) false)
          (set `self.ElapsedTime` 0.0))))))