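; Actor component that makes its owner rise, hover with a bobbing motion and descend once StartFloating is called.
; Tick lifts the owner by FloatingSpeed per frame up to the target height, then applies a sine offset around it until the duration expires.
; It then lowers the owner to the Z captured at BeginPlay.
; Movement is not delta-scaled or swept, and ReachingHeight is never reset between floats.
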(event `self.ReceiveBeginPlay`
  (set `self.InitialLocation` (`Actor.K2_GetActorLocation` (`self.GetOwner`))))

(event `self.ReceiveTick`
  (params (DeltaSeconds :type "Float (single-precision)"))
  (bind (_initiallocation_x _initiallocation_y _initiallocation_z) (`KismetMathLibrary.BreakVector` (`self.InitialLocation`)))
  (bind (_initiallocation_x_2 _initiallocation_y_2 _initiallocation_z_2) (`KismetMathLibrary.BreakVector` (`self.InitialLocation`)))
  (bind (_initiallocation_x_3 _initiallocation_y_3 _initiallocation_z_3) (`KismetMathLibrary.BreakVector` (`self.InitialLocation`)))
  (bind (_returnvalue_x _returnvalue_y _returnvalue_z) (`KismetMathLibrary.BreakVector` (`Actor.K2_GetActorLocation` (`self.GetOwner`))))
  (bind (_returnvalue_x_2 _returnvalue_y_2 _returnvalue_z_2) (`KismetMathLibrary.BreakVector` (`Actor.K2_GetActorLocation` (`self.GetOwner`))))
  (bind (_returnvalue_x_3 _returnvalue_y_3 _returnvalue_z_3) (`KismetMathLibrary.BreakVector` (`Actor.K2_GetActorLocation` (`self.GetOwner`))))
  (if (`self.bFloating`)
    (bind _output_get (set `self.ElapsedTime` (+ DeltaSeconds (`self.ElapsedTime`))))
    (if (< _output_get (`self.FloatingDuration`))
      (if (`self.bReachingHeight`)
        (`Actor.K2_SetActorLocation` (`self.GetOwner`) (`KismetMathLibrary.MakeVector` _initiallocation_x_3 _initiallocation_y_3 (+ _initiallocation_z_3 (* (`KismetMathLibrary.DegSin` (* (`self.ElapsedTime`) (`self.FloatingFrequency`) 360.0)) (`self.FloatingAmplitude`)) (`self.FloatingHeight`))) false false)
        (else
          (`Actor.K2_SetActorLocation` (`self.GetOwner`) (`KismetMathLibrary.MakeVector` _returnvalue_x _returnvalue_y (+ _returnvalue_z (`self.FloatingSpeed`))) false false)
          (set `self.bReachingHeight` (<= (`self.FloatingHeight`) (- _returnvalue_z_2 _initiallocation_z_2)))))
      (else
        (`Actor.K2_SetActorLocation` (`self.GetOwner`) (`KismetMathLibrary.MakeVector` _returnvalue_x_3 _returnvalue_y_3 (- _returnvalue_z_3 (`self.FloatingSpeed`))) false false)
        (set `self.bFloating` (> (- _returnvalue_z_3 _initiallocation_z) 0.0))))))

(fn `StartFloating`
  (params (Amplitude :type "Float (double-precision)") (Duration :type "Float (double-precision)") (Freqency :type "Float (double-precision)") (Height :type "Float (double-precision)"))
  (set `self.bFloating` true)
  (set `self.ElapsedTime` 0.0)
  (set `self.FloatingAmplitude` Amplitude)
  (set `self.FloatingDuration` Duration)
  (set `self.FloatingFrequency` Freqency)
  (set `self.FloatingHeight` Height))