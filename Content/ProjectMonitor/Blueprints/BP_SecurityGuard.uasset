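; BP_SecurityGuard is a security guard pawn that walks a one-way route through an ordered array of destination actors.
; A recursive Patrol event starts on BeginPlay, advances the index after each successful AIMoveTo, and sets Arrived once the array is exhausted.
; A failed move has no handler, so the route stops there.
; GetSocket exposes world-space transforms of sockets on the guard's Weapon.
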(event `self.ReceiveBeginPlay`
  (`self.Patrol`))

(event `Patrol`
  (if (< (`self.DestinationIndex`) (`KismetArrayLibrary.Array_Length` (`self.DestinationArray`)))
    (`|AIMoveTo` self (0.0 0.0 0.0) (`|GetArrayItem` (`self.DestinationArray`) (`self.DestinationIndex`))
      (:`OnSuccess`
        (`/Engine/EditorBlueprintResources/StandardMacros.IncrementInt` (`self.DestinationIndex`)
          (:`  `
            (`self.Patrol`)))))
    (else
      (set `self.bArrived` true))))

(fn `GetSocket`
  (params (SocketName :type Name))
  (returns (SocketTransform :type "Transform Structure"))
  (return (`SceneComponent.GetSocketTransform` (`self.Weapon`) SocketName "RTS_World")))

(fn `UserConstructionScript`)