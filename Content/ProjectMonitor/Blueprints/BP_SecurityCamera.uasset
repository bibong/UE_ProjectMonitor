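; BP_SecurityCamera is a security camera that takes player axis input for turning and zoom.
; Input events pass axis values to TurnUp, TurnRight and Zoom.
; BeginPlay builds an array of weighted dynamic post-process materials for noise and night vision, both starting at zero weight, then toggles noise.
; TogglePostProcess flips the noise blendable's weight through a FlipFlop and has no night vision case.
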(event `InputAxis|TurnUp`
  (params (AxisValue :type "Float (single-precision)"))
  ;[1 1 1] Input
  (`self.TurnUp` AxisValue))

(event `InputAxis|TurnRight`
  (params (AxisValue :type "Float (single-precision)"))
  ;[1 1 1] Input
  (`self.TurnRight` AxisValue))

(event `InputAxis|Zoom`
  (params (AxisValue :type "Float (single-precision)"))
  ;[1 1 1] Input
  (`self.Zoom` AxisValue))

(event `self.ReceiveBeginPlay`
  (`|ExecutionSequence`
    (:`then_0`
      (bind _returnvalue (`KismetMaterialLibrary.CreateDynamicMaterialInstance` "/Game/ProjectMonitor/PostProcess/M_Noise.M_Noise"))
      (`KismetArrayLibrary.Array_Add` (`self.PostProcessMaterialArray`) (make `WeightedBlendable` 0.0 _returnvalue)))
    (:`then_1`
      (bind _returnvalue_2 (`KismetMaterialLibrary.CreateDynamicMaterialInstance` "/Game/ProjectMonitor/PostProcess/M_NightVision.M_NightVision"))
      (`KismetArrayLibrary.Array_Add` (`self.PostProcessMaterialArray`) (make `WeightedBlendable` 0.0 _returnvalue_2)))
    (:`then_2`
      (set `self.PostProcessMaterialArray` (`self.PostProcessMaterialArray`))
      (`self.Event TogglePostProcess` "NewEnumerator0"))))

(event `Event TogglePostProcess`
  (params (PostProcess :type "/Game/ProjectMonitor/Blueprints/E_PostProcess Enum" :default "NewEnumerator0"))
  (switch `/Game/ProjectMonitor/Blueprints/E_PostProcess` PostProcess
    (:`NewEnumerator0`
      (bind _isa (`/Engine/EditorBlueprintResources/StandardMacros.FlipFlop`)
        (:`A`
          _)
        (:`B`
          _))
      (setmembers `WeightedBlendable` :`StructRef` (`|GetArrayItem` (`self.PostProcessMaterialArray`)) :`Weight` (`KismetMathLibrary.SelectFloat` 1.0 0.0 _isa)))))

(fn `UserConstructionScript`)